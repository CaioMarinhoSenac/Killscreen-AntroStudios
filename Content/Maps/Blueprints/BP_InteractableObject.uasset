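; Interactable world object that the player toggles interaction on with IA_Interact while inside its Box trigger.
; Box overlaps use IsPlayerMessage to identify the player, then show or hide the prompt widget and enable or disable input.
; The input uncrouches the interacting Character and calls BeginInteraction or EndInteraction based on IsInteracting.
; Both events clear CanSwitchInteraction to block further toggling, and nothing in this Blueprint sets it back.
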(event OnComponentBeginOverlap(Box)
  (params (OverlappedComponent :type Primitive%20Component%20Object%20Reference) (OtherActor :type Actor%20Object%20Reference) (OtherComp :type Primitive%20Component%20Object%20Reference) (OtherBodyIndex :type Integer) (bFromSweep :type Boolean) (SweepResult :type Hit%20Result%20Structure%20%28by%20ref%29))
  (bind _output_get (Variables|Default|SetInteractingActor OtherActor))
  (bind _true_false (Class|BPICharacter|IsPlayer(Message) _output_get))
  (if _true_false
    (Rendering|SetVisibility (Variables|Default|GetWidget) true false)
    (Input|EnableInput (Game|GetPlayerController 0))))

(event OnComponentEndOverlap(Box)
  (params (OverlappedComponent :type Primitive%20Component%20Object%20Reference) (OtherActor :type Actor%20Object%20Reference) (OtherComp :type Primitive%20Component%20Object%20Reference) (OtherBodyIndex :type Integer))
  (bind _true_false (Class|BPICharacter|IsPlayer(Message) OtherActor))
  (if _true_false
    (Rendering|SetVisibility (Variables|Default|GetWidget) false false)
    (Input|DisableInput (Game|GetPlayerController 0))))

(event Custom|BeginInteraction
  (Variables|Default|SetIsInteracting true)
  (Rendering|SetVisibility (Variables|Default|GetWidget) false false)
  (bind _ascharacter (Utilities|Casting|CastToCharacter (Variables|Default|GetInteractingActor)))
  (Variables|Default|SetCharacter _ascharacter)
  (Variables|Default|SetCanSwitchInteraction false))

(event Custom|EndInteraction
  (Variables|Default|SetIsInteracting false)
  (Variables|Default|SetCanSwitchInteraction false))

(event Input|EnhancedActionEvents|EnhancedInputActionIA_Interact
  (params (ActionValue :type Boolean) (ElapsedSeconds :type Float%20%28double-precision%29) (TriggeredSeconds :type Float%20%28double-precision%29) (InputAction :type Input%20Action%20Object%20Reference :default "/Game/Maps/Input/Actions/IA_Interact.IA_Interact"))
  (:Started
    (if (Variables|Default|GetCanSwitchInteraction)
      (bind _ascharacter (Utilities|Casting|CastToCharacter (Variables|Default|GetInteractingActor)))
      (Character|UnCrouch _ascharacter)
      (if (Variables|Default|GetIsInteracting)
        (CallFunction|EndInteraction)
        (else
          (CallFunction|BeginInteraction))))))

(fn ConstructionScript)
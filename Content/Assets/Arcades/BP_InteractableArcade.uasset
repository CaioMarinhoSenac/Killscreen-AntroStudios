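; Interactable arcade machine built on a parent interactable class, highlighting its buttons through custom depth while an actor overlaps it.
; Beginning interaction disables the character's movement message, eases the character to the PlayPosition component and plays the gaming montage, moving the highlight from buttons to base.
; Ending interaction stops the montage on the BP_Garota actor, restores highlight and movement, shows the widget and re-enables interaction switching.
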(event EventBeginInteraction
  (bind _playposition (Variables|Default|GetPlayPosition))
  (bind _character (Variables|Default|GetCharacter))
  (|CallParentFunction)
  (Class|BPICharacter|ToggleMovement(Message) _character false)
  (Components|MoveComponentTo (Variables|/Script/Engine.Actor|GetRootComponent _character) (+ (Math|Vector|MakeVector 0.0 0.0 (Variables|/Script/Engine.CapsuleComponent|GetCapsuleHalfHeight (Variables|/Script/Engine.Character|GetCapsuleComponent _character))) (Transformation|GetWorldLocation _playposition)) (Transformation|GetWorldRotation _playposition) true true 0.5 false)
  (Animation|PlayAnimMontage (Variables|Default|GetCharacter) "/Game/Characters/Personagens/Garota/Animations/AM_Gaming.AM_Gaming" 1.0 "None")
  (Rendering|SetRenderCustomDepth (Variables|Default|GetBotões) false)
  (Rendering|SetRenderCustomDepth (Variables|Default|GetBase) true))

(event EventEndInteraction
  (|CallParentFunction)
  (bind _returnvalue (Actor|GetActorOfClass "/Game/Characters/Personagens/Garota/BP_Garota.BP_Garota_C"))
  (Animation|StopAnimMontage _returnvalue "/Game/Characters/Personagens/Garota/Animations/AM_Gaming.AM_Gaming")
  (Rendering|SetRenderCustomDepth (Variables|Default|GetBotões) true)
  (Rendering|SetRenderCustomDepth (Variables|Default|GetBase) false)
  (Class|BPICharacter|ToggleMovement(Message) (Variables|Default|GetCharacter) true)
  (Rendering|SetVisibility (Variables|Default|GetWidget) true false)
  (Variables|Default|SetCanSwitchInteraction true))

(event Collision|EventActorBeginOverlap
  (params (OtherActor :type Actor%20Object%20Reference))
  (|CallParentFunction OtherActor)
  (Rendering|SetRenderCustomDepth (Variables|Default|GetBotões) true))

(event Collision|EventActorEndOverlap
  (params (OtherActor :type Actor%20Object%20Reference))
  (|CallParentFunction OtherActor)
  (Rendering|SetRenderCustomDepth (Variables|Default|GetBotões) false))

(fn ConstructionScript
  (|CallParentFunction))
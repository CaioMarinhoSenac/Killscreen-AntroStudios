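; Formation of ten Space Invaders-style enemies in a single actor for the SpaceWar arcade game, each a Paper2D sprite with its own collision box.
; Delay loops gated by CanControl step the root sideways per ChangeSide, drop it when Down is set, and fire projectiles from a random sprite's position.
; A player projectile overlap calls Death, which spawns an explosion, destroys that sprite, box and projectile, and adds score to BP_GameSpaceWar.
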(event OnComponentBeginOverlap(Box1)
  (params (OverlappedComponent :type Primitive%20Component%20Object%20Reference) (OtherActor :type Actor%20Object%20Reference) (OtherComp :type Primitive%20Component%20Object%20Reference) (OtherBodyIndex :type Integer) (bFromSweep :type Boolean) (SweepResult :type Hit%20Result%20Structure%20%28by%20ref%29))
  (bind _asbp_player_projetil_space_war (Utilities|Casting|CastToBP_PlayerProjetilSpaceWar OtherActor))
  (CallFunction|Death _asbp_player_projetil_space_war (Variables|Default|GetPaperSprite1) (Variables|Default|GetBox1)))

(event OnComponentBeginOverlap(Box4)
  (params (OverlappedComponent :type Primitive%20Component%20Object%20Reference) (OtherActor :type Actor%20Object%20Reference) (OtherComp :type Primitive%20Component%20Object%20Reference) (OtherBodyIndex :type Integer) (bFromSweep :type Boolean) (SweepResult :type Hit%20Result%20Structure%20%28by%20ref%29))
  (bind _asbp_player_projetil_space_war (Utilities|Casting|CastToBP_PlayerProjetilSpaceWar OtherActor))
  (CallFunction|Death _asbp_player_projetil_space_war (Variables|Default|GetPaperSprite4) (Variables|Default|GetBox4)))

(event OnComponentBeginOverlap(Box5)
  (params (OverlappedComponent :type Primitive%20Component%20Object%20Reference) (OtherActor :type Actor%20Object%20Reference) (OtherComp :type Primitive%20Component%20Object%20Reference) (OtherBodyIndex :type Integer) (bFromSweep :type Boolean) (SweepResult :type Hit%20Result%20Structure%20%28by%20ref%29))
  (bind _asbp_player_projetil_space_war (Utilities|Casting|CastToBP_PlayerProjetilSpaceWar OtherActor))
  (CallFunction|Death _asbp_player_projetil_space_war (Variables|Default|GetPaperSprite5) (Variables|Default|GetBox5)))

(event OnComponentBeginOverlap(Box3)
  (params (OverlappedComponent :type Primitive%20Component%20Object%20Reference) (OtherActor :type Actor%20Object%20Reference) (OtherComp :type Primitive%20Component%20Object%20Reference) (OtherBodyIndex :type Integer) (bFromSweep :type Boolean) (SweepResult :type Hit%20Result%20Structure%20%28by%20ref%29))
  (bind _asbp_player_projetil_space_war (Utilities|Casting|CastToBP_PlayerProjetilSpaceWar OtherActor))
  (CallFunction|Death _asbp_player_projetil_space_war (Variables|Default|GetPaperSprite3) (Variables|Default|GetBox3)))

(event OnComponentBeginOverlap(Box2)
  (params (OverlappedComponent :type Primitive%20Component%20Object%20Reference) (OtherActor :type Actor%20Object%20Reference) (OtherComp :type Primitive%20Component%20Object%20Reference) (OtherBodyIndex :type Integer) (bFromSweep :type Boolean) (SweepResult :type Hit%20Result%20Structure%20%28by%20ref%29))
  (bind _asbp_player_projetil_space_war (Utilities|Casting|CastToBP_PlayerProjetilSpaceWar OtherActor))
  (CallFunction|Death _asbp_player_projetil_space_war (Variables|Default|GetPaperSprite2) (Variables|Default|GetBox2)))

(event OnComponentBeginOverlap(Box9)
  (params (OverlappedComponent :type Primitive%20Component%20Object%20Reference) (OtherActor :type Actor%20Object%20Reference) (OtherComp :type Primitive%20Component%20Object%20Reference) (OtherBodyIndex :type Integer) (bFromSweep :type Boolean) (SweepResult :type Hit%20Result%20Structure%20%28by%20ref%29))
  (bind _asbp_player_projetil_space_war (Utilities|Casting|CastToBP_PlayerProjetilSpaceWar OtherActor))
  (CallFunction|Death _asbp_player_projetil_space_war (Variables|Default|GetPaperSprite9) (Variables|Default|GetBox9)))

(event OnComponentBeginOverlap(Box10)
  (params (OverlappedComponent :type Primitive%20Component%20Object%20Reference) (OtherActor :type Actor%20Object%20Reference) (OtherComp :type Primitive%20Component%20Object%20Reference) (OtherBodyIndex :type Integer) (bFromSweep :type Boolean) (SweepResult :type Hit%20Result%20Structure%20%28by%20ref%29))
  (bind _asbp_player_projetil_space_war (Utilities|Casting|CastToBP_PlayerProjetilSpaceWar OtherActor))
  (CallFunction|Death _asbp_player_projetil_space_war (Variables|Default|GetPaperSprite10) (Variables|Default|GetBox10)))

(event OnComponentBeginOverlap(Box6)
  (params (OverlappedComponent :type Primitive%20Component%20Object%20Reference) (OtherActor :type Actor%20Object%20Reference) (OtherComp :type Primitive%20Component%20Object%20Reference) (OtherBodyIndex :type Integer) (bFromSweep :type Boolean) (SweepResult :type Hit%20Result%20Structure%20%28by%20ref%29))
  (bind _asbp_player_projetil_space_war (Utilities|Casting|CastToBP_PlayerProjetilSpaceWar OtherActor))
  (CallFunction|Death _asbp_player_projetil_space_war (Variables|Default|GetPaperSprite6) (Variables|Default|GetBox6)))

(event OnComponentBeginOverlap(Box7)
  (params (OverlappedComponent :type Primitive%20Component%20Object%20Reference) (OtherActor :type Actor%20Object%20Reference) (OtherComp :type Primitive%20Component%20Object%20Reference) (OtherBodyIndex :type Integer) (bFromSweep :type Boolean) (SweepResult :type Hit%20Result%20Structure%20%28by%20ref%29))
  (bind _asbp_player_projetil_space_war (Utilities|Casting|CastToBP_PlayerProjetilSpaceWar OtherActor))
  (CallFunction|Death _asbp_player_projetil_space_war (Variables|Default|GetPaperSprite7) (Variables|Default|GetBox7)))

(event OnComponentBeginOverlap(Box8)
  (params (OverlappedComponent :type Primitive%20Component%20Object%20Reference) (OtherActor :type Actor%20Object%20Reference) (OtherComp :type Primitive%20Component%20Object%20Reference) (OtherBodyIndex :type Integer) (bFromSweep :type Boolean) (SweepResult :type Hit%20Result%20Structure%20%28by%20ref%29))
  (bind _asbp_player_projetil_space_war (Utilities|Casting|CastToBP_PlayerProjetilSpaceWar OtherActor))
  (CallFunction|Death _asbp_player_projetil_space_war (Variables|Default|GetPaperSprite8) (Variables|Default|GetBox8)))

(event EventBeginPlay
  (Utilities|FlowControl|Sequence
    (:then_0
      (|Moviment))
    (:then_1
      (Utilities|FlowControl|Delay 1.5)
      (|Shoot))))

(fn ConstructionScript)

(fn Death
  (params (Projetil :type Actor%20Object%20Reference) (PaperSprite :type Actor%20Component%20Object%20Reference) (BoxCollision :type Actor%20Component%20Object%20Reference))
  (Game|SpawnActorfromClass "/Game/Assets/Arcades/Jogos/SpaceInvaders/Assets/BP_EnemySpaceWarExplosion.BP_EnemySpaceWarExplosion_C" (Math|Transform|MakeTransform (+ (.location (Transformation|GetWorldTransform (Variables|/Script/Engine.Actor|GetRootComponent Projetil))) "0.000000,0.000000,10.000000") "0, 0, 0" "1.000000,1.000000,1.000000") "Undefined" "MultiplyWithRoot" 0 0)
  (Actor|DestroyActor Projetil)
  (Components|DestroyComponent PaperSprite)
  (Components|DestroyComponent BoxCollision)
  (bind _returnvalue (Actor|GetActorOfClass "/Game/Assets/Arcades/Jogos/SpaceInvaders/BP_GameSpaceWar.BP_GameSpaceWar_C"))
  (Default|SetScore _returnvalue (+ (Variables|/Game/Assets/Arcades/Jogos/SpaceInvaders/BP_GameSpaceWar.BP_GameSpaceWar_C|GetScore _returnvalue) (Variables|Default|GetScoreAmount))))
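; Player ship for the Space Invaders arcade minigame, controlled by keyboard input.
; W spawns a projectile actor at the arrow component's transform, with a short delay-gated flag limiting the fire rate.
; A and D nudge the collision component sideways by a fixed step on each press, using an instant MoveComponentTo rather than continuous axis movement.
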(event Input|KeyboardEvents|D
  (params (Key :type Key%20Structure :default "None"))
  (bind _playercollision (Variables|Default|GetPlayerCollision))
  (:Pressed
    (Components|MoveComponentTo _playercollision (+ (Variables|/Script/Engine.SceneComponent|GetRelativeLocation _playercollision) "-7.000000,0.000000,0.000000") "0, 0, 0" false false 0.0 false)))

(event Input|KeyboardEvents|W
  (params (Key :type Key%20Structure :default "None"))
  (:Pressed
    (if (Variables|Combat|GetCanShoot)
      (Game|SpawnActorfromClass "/Game/Assets/Arcades/Jogos/SpaceInvaders/Assets/BP_ProjeteisSpaceInvaders.BP_ProjeteisSpaceInvaders_C" (Transformation|GetWorldTransform (Variables|Default|GetArrow)) "AlwaysSpawn" "MultiplyWithRoot" 0 0)
      (Variables|Combat|SetCanShoot false)
      (Utilities|FlowControl|Delay 0.3)
      (Variables|Combat|SetCanShoot true))))

(event Input|KeyboardEvents|A
  (params (Key :type Key%20Structure :default "None"))
  (bind _playercollision (Variables|Default|GetPlayerCollision))
  (:Pressed
    (Components|MoveComponentTo _playercollision (+ (Variables|/Script/Engine.SceneComponent|GetRelativeLocation _playercollision) "7.000000,0.000000,0.000000") "0, 0, 0" false false 0.0 false)))

(fn ConstructionScript)
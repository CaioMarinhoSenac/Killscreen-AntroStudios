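; Player ship for the Space War arcade minigame, a Space Invaders-style shooter played on an in-world cabinet.
; While CanControl is set, A/D presses nudge the collision sideways in fixed steps and W fires a projectile from the Arrow, gated by a cooldown.
; Enemy projectile hits decrement life on BP_GameSpaceWar and spawn an explosion; enemy contact zeroes it.
; Shot sounds play at the cabinet screen, hit sounds at BP_Garota.
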(event OnComponentBeginOverlap(PlayerCollision)
  (params (OverlappedComponent :type Primitive%20Component%20Object%20Reference) (OtherActor :type Actor%20Object%20Reference) (OtherComp :type Primitive%20Component%20Object%20Reference) (OtherBodyIndex :type Integer) (bFromSweep :type Boolean) (SweepResult :type Hit%20Result%20Structure%20%28by%20ref%29))
  (bind _gamespacewar (Variables|Components|GetGameSpaceWar))
  (Utilities|Casting|CastToBP_EnemyProjetilSpaceWar OtherActor
    (:then
      (Utilities|FlowControl|Sequence
        (:then_0
          (Actor|DestroyActor OtherActor)
          (Default|SetPlayerLife _gamespacewar (- (Variables|/Game/Assets/Arcades/Jogos/SpaceInvaders/BP_GameSpaceWar.BP_GameSpaceWar_C|GetPlayerLife _gamespacewar) 1)))
        (:then_1
          (Game|SpawnActorfromClass "/Game/Assets/Arcades/Jogos/SpaceInvaders/Assets/BP_EnemyProjetilSpaceWarExplosion.BP_EnemyProjetilSpaceWarExplosion_C" (Math|Transform|MakeTransform (+ (Transformation|GetWorldLocation (Variables|Default|GetPlayer_Sprite)) "0.000000,0.000000,10.000000") "0, 0, 0" "1.000000,1.000000,1.000000") "AlwaysSpawn" "MultiplyWithRoot" 0 0)
          (bind _returnvalue (Actor|GetActorOfClass "/Game/Characters/Personagens/Garota/BP_Garota.BP_Garota_C"))
          (Audio|PlaySoundatLocation "/Game/Assets/Arcades/Jogos/SpaceInvaders/Audio/HIT_PLAYER.HIT_PLAYER" (Transformation|GetWorldLocation (Variables|/Script/Engine.Actor|GetRootComponent _returnvalue)) "0, 0, 0" 1.0 1.0 0.0 0 0 0 0))))
    (:CastFailed
      (Utilities|Casting|CastToBP_EnemySpaceWar OtherActor)
      (bind _returnvalue_2 (Actor|GetActorOfClass "/Game/Assets/Arcades/Jogos/SpaceInvaders/BP_GameSpaceWar.BP_GameSpaceWar_C"))
      (Default|SetPlayerLife _returnvalue_2))))

(event EventBeginPlay
  (bind _returnvalue (Actor|GetActorOfClass "/Game/Assets/Arcades/Jogos/SpaceInvaders/BP_GameSpaceWar.BP_GameSpaceWar_C"))
  (bind _output_get (Variables|Components|SetGameSpaceWar _returnvalue))
  (Variables|Components|SetArcade%20Space%20War (Variables|/Game/Assets/Arcades/Jogos/SpaceInvaders/BP_GameSpaceWar.BP_GameSpaceWar_C|GetArcadeSpaceWar _output_get)))

(event Input|KeyboardEvents|D
  (params (Key :type Key%20Structure :default "None"))
  (:Pressed
    (if (Variables|Default|GetCanControl)
      (Utilities|String|Right))))

(event Input|KeyboardEvents|W
  (params (Key :type Key%20Structure :default "None"))
  (:Pressed
    (if (and (Variables|Default|GetCanControl) (Variables|Combat|GetCanShoot))
      (|Shoot))))

(event Input|KeyboardEvents|A
  (params (Key :type Key%20Structure :default "None"))
  (:Pressed
    (if (Variables|Default|GetCanControl)
      (Utilities|String|Left))))

(fn ConstructionScript)
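; Space Invaders-style arcade cabinet interactable that lets the player play the Space War minigame on its screen.
; On interaction it starts BP_GameSpaceWar, moves possession to BP_PlayerSpaceWar, blends the view from the Character to the cabinet, and swaps the screen to the game material.
; Ending interaction returns possession to the Character, stops its win/lose montages, then restores the start screen and ends the game after a delay.
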(event Collision|EventActorBeginOverlap
  (params (OtherActor :type Actor%20Object%20Reference))
  (|CallParentFunction OtherActor) ; This node is disabled and will not be called.\nDrag off pins to build functionality.
)

(event EventBeginInteraction
  (|CallParentFunction)
  (Utilities|FlowControl|Delay 1.0)
  (Pawn|UnPossess (Game|GetPlayerController 0))
  (bind _returnvalue (Actor|GetActorOfClass "/Game/Assets/Arcades/Jogos/SpaceInvaders/BP_GameSpaceWar.BP_GameSpaceWar_C"))
  (Default|PlayGame _returnvalue)
  (bind _returnvalue_2 (Actor|GetActorOfClass "/Game/Assets/Arcades/Jogos/SpaceInvaders/Personagens/BP_PlayerSpaceWar.BP_PlayerSpaceWar_C"))
  (Pawn|Possess (Game|GetPlayerController 0) _returnvalue_2)
  (Game|Player|SetViewTargetwithBlend (Game|GetPlayerController 0) (Variables|Default|GetCharacter) 0.0 "VTBlend_Linear" 0.0 false)
  (Game|Player|SetViewTargetwithBlend (Game|GetPlayerController 0) self 0.5 "VTBlend_Cubic" 0.0 false)
  (Rendering|Material|SetMaterial (Variables|Default|GetTela) 0 "/Game/Assets/Arcades/Jogos/SpaceInvaders/Texturas/M_GameSpacewar.M_GameSpacewar")
  (Utilities|FlowControl|Delay 2.0)
  (Variables|Default|SetCanSwitchInteraction true))

(event EventEndInteraction
  (bind _character (Variables|Default|GetCharacter))
  (|CallParentFunction)
  (Pawn|UnPossess (Game|GetPlayerController 0))
  (Pawn|Possess (Game|GetPlayerController 0) _character)
  (Animation|StopAnimMontage _character "/Game/Characters/Personagens/Garota/Animations/AM_Winning.AM_Winning")
  (Animation|StopAnimMontage _character "/Game/Characters/Personagens/Garota/Animations/AM_LoosingMatch.AM_LoosingMatch")
  (Utilities|FlowControl|Delay 2.0)
  (Rendering|Material|SetMaterial (Variables|Default|GetTela) 0 "/Game/Assets/Arcades/Jogos/SpaceInvaders/Tela/TelaStartSpaceWar.TelaStartSpaceWar")
  (bind _returnvalue (Actor|GetActorOfClass "/Game/Assets/Arcades/Jogos/SpaceInvaders/BP_GameSpaceWar.BP_GameSpaceWar_C"))
  (Default|EndGame _returnvalue)
  (Variables|Default|SetIsInteracting false)
  (Variables|Default|SetCanSwitchInteraction true))

(fn ConstructionScript
  (|CallParentFunction))
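; Game manager actor for the Space War arcade minigame, a Space Invaders-style match.
; PlayGame respawns player and enemy actors and resets state, while EndGame destroys them and resets.
; Score and life setters trigger win or lose, which show text, play a character montage, freeze controls and end the arcade interaction after a delay.
; Boundary overlaps flip the enemies' direction, step them down, and explode stray projectiles.
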(event OnComponentBeginOverlap(Direita)
  (params (OverlappedComponent :type Primitive%20Component%20Object%20Reference) (OtherActor :type Actor%20Object%20Reference) (OtherComp :type Primitive%20Component%20Object%20Reference) (OtherBodyIndex :type Integer) (bFromSweep :type Boolean) (SweepResult :type Hit%20Result%20Structure%20%28by%20ref%29))
  ;[1 1 1] Collisors
  (bind _asbp_enemy_space_war (Utilities|Casting|CastToBP_EnemySpaceWar OtherActor))
  (Variables|/Game/Assets/Arcades/Jogos/SpaceInvaders/Personagens/BP_EnemySpaceWar.BP_EnemySpaceWar_C|SetChangeSide _asbp_enemy_space_war false)
  (Variables|/Game/Assets/Arcades/Jogos/SpaceInvaders/Personagens/BP_EnemySpaceWar.BP_EnemySpaceWar_C|SetDown _asbp_enemy_space_war true))

(event OnComponentBeginOverlap(Esquerda)
  (params (OverlappedComponent :type Primitive%20Component%20Object%20Reference) (OtherActor :type Actor%20Object%20Reference) (OtherComp :type Primitive%20Component%20Object%20Reference) (OtherBodyIndex :type Integer) (bFromSweep :type Boolean) (SweepResult :type Hit%20Result%20Structure%20%28by%20ref%29))
  ;[1 1 1] Collisors
  (bind _asbp_enemy_space_war (Utilities|Casting|CastToBP_EnemySpaceWar OtherActor))
  (Variables|/Game/Assets/Arcades/Jogos/SpaceInvaders/Personagens/BP_EnemySpaceWar.BP_EnemySpaceWar_C|SetChangeSide _asbp_enemy_space_war true)
  (Variables|/Game/Assets/Arcades/Jogos/SpaceInvaders/Personagens/BP_EnemySpaceWar.BP_EnemySpaceWar_C|SetDown _asbp_enemy_space_war true))

(event OnComponentBeginOverlap(Cima)
  (params (OverlappedComponent :type Primitive%20Component%20Object%20Reference) (OtherActor :type Actor%20Object%20Reference) (OtherComp :type Primitive%20Component%20Object%20Reference) (OtherBodyIndex :type Integer) (bFromSweep :type Boolean) (SweepResult :type Hit%20Result%20Structure%20%28by%20ref%29))
  ;[1 1 1] Collisors
  (bind _asbp_player_projetil_space_war (Utilities|Casting|CastToBP_PlayerProjetilSpaceWar OtherActor))
  (Game|SpawnActorfromClass "/Game/Assets/Arcades/Jogos/SpaceInvaders/Assets/BP_PlayerProjetilSpaceWarExplosion.BP_PlayerProjetilSpaceWarExplosion_C" (Math|Transform|MakeTransform (.location (Transformation|GetRelativeTransform (Variables|/Script/Engine.Actor|GetRootComponent OtherActor))) "0, 0, 0" "1.000000,1.000000,1.000000") "Undefined" "MultiplyWithRoot" 0 0)
  (Actor|DestroyActor _asbp_player_projetil_space_war))

(event OnComponentBeginOverlap(Baixo)
  (params (OverlappedComponent :type Primitive%20Component%20Object%20Reference) (OtherActor :type Actor%20Object%20Reference) (OtherComp :type Primitive%20Component%20Object%20Reference) (OtherBodyIndex :type Integer) (bFromSweep :type Boolean) (SweepResult :type Hit%20Result%20Structure%20%28by%20ref%29))
  ;[1 1 1] Collisors
  (bind _asbp_enemy_projetil_space_war (Utilities|Casting|CastToBP_EnemyProjetilSpaceWar OtherActor))
  (Game|SpawnActorfromClass "/Game/Assets/Arcades/Jogos/SpaceInvaders/Assets/BP_EnemyProjetilSpaceWarExplosion.BP_EnemyProjetilSpaceWarExplosion_C" (Math|Transform|MakeTransform (+ (.location (Transformation|GetRelativeTransform (Variables|/Script/Engine.Actor|GetRootComponent OtherActor))) "0.000000,0.000000,7.000000") "0, 0, 0" "1.000000,1.000000,1.000000") "Undefined" "MultiplyWithRoot" 0 0)
  (Actor|DestroyActor _asbp_enemy_projetil_space_war))

(event Custom|PlayGame
  (bind _enemyspawn (Variables|Default|GetEnemySpawn))
  (bind _playerspawn (Variables|Default|GetPlayerSpawn))
  ;[1 1 1] Play or End Game Match
  (bind _player (Variables|Personagens|GetPlayer)
    (:then
      (Actor|DestroyActor _player))
    (:else
      _))
  (bind _enemies (Variables|Personagens|GetEnemies)
    (:then
      (Actor|DestroyActor _enemies))
    (:else
      _))
  (bind _returnvalue (Game|SpawnActorfromClass "/Game/Assets/Arcades/Jogos/SpaceInvaders/Personagens/BP_PlayerSpaceWar.BP_PlayerSpaceWar_C" (Math|Transform|MakeTransform (Transformation|GetWorldLocation _playerspawn) (Transformation|GetWorldRotation _playerspawn) "1.000000,1.000000,1.000000") "Undefined" "MultiplyWithRoot" 0 0))
  (Variables|Personagens|SetPlayer _returnvalue)
  (bind _returnvalue_2 (Game|SpawnActorfromClass "/Game/Assets/Arcades/Jogos/SpaceInvaders/Personagens/BP_EnemySpaceWar.BP_EnemySpaceWar_C" (Math|Transform|MakeTransform (Transformation|GetWorldLocation _enemyspawn) (Transformation|GetWorldRotation _enemyspawn) "1.000000,1.000000,1.000000") "Undefined" "MultiplyWithRoot" 0 0))
  (Variables|Personagens|SetEnemies _returnvalue_2)
  (bind _returnvalue_3 (Actor|GetActorOfClass "/Game/Assets/Arcades/Jogos/SpaceInvaders/BP_ArcadeSpaceWar.BP_ArcadeSpaceWar_C"))
  (Variables|Components|SetArcadeSpaceWar _returnvalue_3)
  (bind _returnvalue_4 (Actor|GetActorOfClass "/Game/Characters/Personagens/Garota/BP_Garota.BP_Garota_C"))
  (Variables|Default|SetCharacter _returnvalue_4)
  (Utilities|ResetVariables))

(event Custom|EndGame
  ;[1 1 1] Play or End Game Match
  (bind _player (Variables|Personagens|GetPlayer)
    (:then
      (Actor|DestroyActor _player))
    (:else
      _))
  (bind _enemies (Variables|Personagens|GetEnemies)
    (:then
      (Actor|DestroyActor _enemies))
    (:else
      _))
  (Utilities|ResetVariables))

(event Custom|LoseGame
  (bind _arcadespacewar (Variables|Components|GetArcadeSpaceWar))
  ;[1 1 1] Win or Lose Game Match
  (Rendering|SetVisibility (Variables|Default|GetGameOverText) true false)
  (Animation|PlayAnimMontage (Variables|Default|GetCharacter) "/Game/Characters/Personagens/Garota/Animations/AM_LoosingMatch.AM_LoosingMatch" 1.0 "None")
  (Audio|Components|Audio|Stop (Variables|/Game/Assets/Arcades/Jogos/SpaceInvaders/BP_ArcadeSpaceWar.BP_ArcadeSpaceWar_C|GetBotõesAudio _arcadespacewar))
  (Variables|/Game/Assets/Arcades/Jogos/SpaceInvaders/Personagens/BP_PlayerSpaceWar.BP_PlayerSpaceWar_C|SetCanControl (Variables|Personagens|GetPlayer) false)
  (Variables|/Game/Assets/Arcades/Jogos/SpaceInvaders/Personagens/BP_EnemySpaceWar.BP_EnemySpaceWar_C|SetCanControl (Variables|Personagens|GetEnemies) false)
  (Utilities|FlowControl|Delay 2.0)
  (Default|EndInteraction _arcadespacewar))

(event Custom|WinGame
  (bind _arcadespacewar (Variables|Components|GetArcadeSpaceWar))
  ;[1 1 1] Win or Lose Game Match
  (Rendering|SetVisibility (Variables|Default|GetWinText) true false)
  (Animation|PlayAnimMontage (Variables|Default|GetCharacter) "/Game/Characters/Personagens/Garota/Animations/AM_Winning.AM_Winning" 1.0 "None")
  (Audio|Components|Audio|Stop (Variables|/Game/Assets/Arcades/Jogos/SpaceInvaders/BP_ArcadeSpaceWar.BP_ArcadeSpaceWar_C|GetBotõesAudio _arcadespacewar))
  (Variables|/Game/Assets/Arcades/Jogos/SpaceInvaders/Personagens/BP_PlayerSpaceWar.BP_PlayerSpaceWar_C|SetCanControl (Variables|Personagens|GetPlayer) false)
  (Variables|/Game/Assets/Arcades/Jogos/SpaceInvaders/Personagens/BP_EnemySpaceWar.BP_EnemySpaceWar_C|SetCanControl (Variables|Personagens|GetEnemies) false)
  (Utilities|FlowControl|Delay 2.0)
  (Default|EndInteraction _arcadespacewar))

(fn ConstructionScript)

(fn SetScore
  (params (NewScore :type Integer))
  (bind _output_get (Variables|Score|SetScore NewScore))
  (Rendering|Components|TextRender|SetText (Variables|Default|GetScorePoints) (Utilities|Text|ToText(Integer) _output_get))
  (if (>= _output_get (Variables|Score|GetScoreGoal))
    (CallFunction|Wingame)))

(fn SetPlayerLife
  (params (NewLife :type Integer))
  (bind _player (Variables|Personagens|GetPlayer))
  (bind _output_get (Variables|Life|SetPlayerLife NewLife))
  (if (<= _output_get 0)
    (Game|SpawnActorfromClass "/Game/Assets/Arcades/Jogos/SpaceInvaders/Assets/BP_PlayerSpaceWarExplosion.BP_PlayerSpaceWarExplosion_C" (Math|Transform|MakeTransform (Transformation|GetWorldLocation (Variables|/Game/Assets/Arcades/Jogos/SpaceInvaders/Personagens/BP_PlayerSpaceWar.BP_PlayerSpaceWar_C|GetPlayer_Sprite _player)) "0, 0, 0" "1.000000,1.000000,1.000000") "Undefined" "MultiplyWithRoot" 0 0)
    (Rendering|Components|Sprite|SetSprite (Variables|/Game/Assets/Arcades/Jogos/SpaceInvaders/Personagens/BP_PlayerSpaceWar.BP_PlayerSpaceWar_C|GetPlayer_Sprite _player) "/Game/Assets/Arcades/Jogos/SpaceInvaders/Assets/PlayerExplosion_Sprite.PlayerExplosion_Sprite")
    (Audio|PlaySoundatLocation "/Game/Assets/Arcades/Jogos/SpaceInvaders/Audio/NAVE_EXPLODINDO_JOGADOR.NAVE_EXPLODINDO_JOGADOR" (Transformation|GetWorldLocation (Variables|/Game/Assets/Arcades/BP_InteractableArcade.BP_InteractableArcade_C|GetTelaVidro (Variables|Components|GetArcadeSpaceWar))) "0, 0, 0" 1.0 1.0 0.0 0 0 0 0)
    (CallFunction|LoseGame)))
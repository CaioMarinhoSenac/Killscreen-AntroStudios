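; Interactable locker Blueprint that a Character uses to hide, extending a parent's overlap and interaction events.
; Overlap toggles custom depth on the locker door as a highlight.
; Beginning interaction disables the character's movement through a message, plays the hide montage and shifts custom depth from door to base.
; Ending interaction restores movement, stops the montage and returns custom depth to the door if the stored character is valid.
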(event EventBeginInteraction
  (|CallParentFunction)
  (bind _ascharacter (Utilities|Casting|CastToCharacter (Variables|Default|GetInteractingActor)))
  (bind _output_get (Variables|Default|SetCharacter _ascharacter))
  (Class|BPICharacter|ToggleMovement(Message) _output_get false)
  (Animation|PlayAnimMontage _output_get "/Game/Characters/Personagens/Garota/Animations/AM_Hide.AM_Hide" 1.0 "None")
  (Rendering|SetRenderCustomDepth (Variables|Default|GetLockerDoor) false)
  (Rendering|SetRenderCustomDepth (Variables|Default|GetLockerBase) true))

(event EventEndInteraction
  (|CallParentFunction)
  (bind _character (Variables|Default|GetCharacter)
    (:then
      (Class|BPICharacter|ToggleMovement(Message) _character true)
      (Animation|StopAnimMontage _character "/Game/Characters/Personagens/Garota/Animations/AM_Hide.AM_Hide")
      (Rendering|SetRenderCustomDepth (Variables|Default|GetLockerDoor) true)
      (Rendering|SetRenderCustomDepth (Variables|Default|GetLockerBase) false))
    (:else)))

(event Collision|EventActorBeginOverlap
  (params (OtherActor :type Actor%20Object%20Reference))
  (|CallParentFunction OtherActor)
  (Rendering|SetRenderCustomDepth (Variables|Default|GetLockerDoor) true))

(event Collision|EventActorEndOverlap
  (params (OtherActor :type Actor%20Object%20Reference))
  (|CallParentFunction OtherActor)
  (Rendering|SetRenderCustomDepth (Variables|Default|GetLockerDoor) false))

(fn ConstructionScript
  (|CallParentFunction))